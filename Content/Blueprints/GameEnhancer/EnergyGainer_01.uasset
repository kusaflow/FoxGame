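; An interactable food pickup, named as an energy gainer, that the fox player character can consume.
; Box overlap sets the fox's interact mode and snap location, and leaving resets the mode.
; Tick polls a game instance flag, then destroys the mesh, clears the flag and marks the food gone.
; That check ignores overlap: CanMushRoomDisapear is set but never read here, so any remaining instance can consume the shared flag.
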(event OnComponentBeginOverlap(Box)
  (params (OverlappedComponent :type Primitive%20Component%20Object%20Reference) (OtherActor :type Actor%20Object%20Reference) (OtherComp :type Primitive%20Component%20Object%20Reference) (OtherBodyIndex :type Integer) (bFromSweep :type Boolean) (SweepResult :type Hit%20Result%20Structure%20%28by%20ref%29))
  (if (Variables|Default|GetisFoodThere)
    (bind _asmain_char_fox (Utilities|Casting|CastTomainChar_Fox OtherActor))
    (Variables|/Script/AnimalStoryGame.mainChar_Fox|SetWhat_to_do_with_interact _asmain_char_fox 1)
    (Variables|/Script/AnimalStoryGame.mainChar_Fox|SetOtherActorLoc_ToSnapLoc _asmain_char_fox (Transformation|GetWorldLocation (Variables|Default|GetBox)))
    (Variables|Default|SetCanMushRoomDisapear true)))

(event OnComponentEndOverlap(Box)
  (params (OverlappedComponent :type Primitive%20Component%20Object%20Reference) (OtherActor :type Actor%20Object%20Reference) (OtherComp :type Primitive%20Component%20Object%20Reference) (OtherBodyIndex :type Integer))
  (bind _asmain_char_fox (Utilities|Casting|CastTomainChar_Fox OtherActor))
  (Variables|/Script/AnimalStoryGame.mainChar_Fox|SetWhat_to_do_with_interact _asmain_char_fox 0)
  (Variables|Default|SetCanMushRoomDisapear false))

(event EventBeginPlay
  (Variables|Default|SetCanMushRoomDisapear true)
  (Variables|Default|SetisFoodThere true))

(event Collision|EventActorBeginOverlap
  (params (OtherActor :type Actor%20Object%20Reference)))

(event EventTick
  (params (DeltaSeconds :type Float%20%28single-precision%29))
  (if (Variables|Default|GetisFoodThere)
    (bind _askusa_game_instance (Utilities|Casting|CastTokusaGameInstance (Game|GetGameInstance)))
    (if (Variables|/Script/AnimalStoryGame.kusaGameInstance|GetbCanDisapearFood _askusa_game_instance)
      (Components|DestroyComponent (Variables|Default|GetStaticMesh))
      (Variables|/Script/AnimalStoryGame.kusaGameInstance|SetbCanDisapearFood _askusa_game_instance false)
      (Variables|Default|SetisFoodThere false))))

(fn ConstructionScript)