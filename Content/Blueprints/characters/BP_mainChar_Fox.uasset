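; BP_mainChar_Fox is the fox main character Blueprint, handling animation state, cinematic playback and a path-revealing scan.
; Each tick it computes local forward velocity for animation and sets the mesh's anim class from AnimInstIdx, either the default fox AnimBP or a rope-opening one.
; Pressing J sets the game instance's show-path flag while a timeline drives the ScanPara collection's radius, then resets both.
; PlayAnimation plays the assigned level sequence.
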(event Custom|rotation
  (bind _rootcomponent (Variables|Transformation|GetRootComponent))
  ;[1 1 1] rotation
  (Variables|Default|SetVelForAnim_MoveFor (.X (Math|Vector|BreakVector (Math|Vector|UnrotateVector (Transformation|GetComponentVelocity _rootcomponent) (Transformation|GetWorldRotation _rootcomponent))))))

(event Custom|resetAnimInstance
  (bind _mesh (Variables|Character|GetMesh))
  ;[1 1 1] AnimInstance Reset
  (switch int (Variables|Default|GetAnimInst_Idx)
    (:Default
      (Class|SkeletalMeshComponent|SetAnimClass _mesh "/Game/Blueprints/characters/Animations/AnimBP_Fox.AnimBP_Fox_C" :!label _label))
    (:0
      (goto _label))
    (:1
      (Class|SkeletalMeshComponent|SetAnimClass _mesh "/Game/Blueprints/characters/Animations/FOX_A_OpeningRopes.FOX_A_OpeningRopes_C"))))

(event EventBeginPlay)

(event Collision|EventActorBeginOverlap
  (params (OtherActor :type Actor%20Object%20Reference)))

(event EventTick
  (params (DeltaSeconds :type Float%20%28single-precision%29))
  (CallFunction|Rotation)
  (CallFunction|ResetAnimInstance))

(event EventPlayAnimation
  (bind _cinemetic (Variables|Default|Getcinemetic))
  ;[1 1 1] playAnimation
  (Utilities|IsValid _cinemetic
    (:Is%20Valid
      (bind _returnvalue (Sequencer|Player|CreateLevelSequencePlayer _cinemetic))
      (Sequencer|Player|Play _returnvalue :!class /Script/MovieScene.MovieSceneSequencePlayer))))

(event Input|KeyboardEvents|J
  (params (Key :type Key%20Structure :default "None"))
  (:Pressed
    (bind _askusa_game_instance (Utilities|Casting|CastTokusaGameInstance (Game|GetGameInstance)))
    (Variables|/Script/AnimalStoryGame.kusaGameInstance|SetbshowPath _askusa_game_instance true)
    (bind _newtrack_0 (Timeline|Timeline_0 PlayFromStart)
      (:Update
        (Rendering|Material|SetScalarParameterValue "/Game/materials/postprocessing/scanEffect/scanPara.scanPara" "radius" _newtrack_0 :!class /Script/Engine.KismetMaterialLibrary))
      (:Finished
        (Variables|/Script/AnimalStoryGame.kusaGameInstance|SetbshowPath _askusa_game_instance false)
        (Rendering|Material|SetScalarParameterValue "/Game/materials/postprocessing/scanEffect/scanPara.scanPara" "radius" 0.0 :!class /Script/Engine.KismetMaterialLibrary)))))

(fn ConstructionScript)